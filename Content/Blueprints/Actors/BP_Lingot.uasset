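; BP_Lingot is an interactable ingot pickup that shows a collection notice on the HUD and then removes itself from the world.
; On LaunchInteract it runs the parent logic, then creates a WB_AddCollectectable widget from its TypeContent and NumberContent.
; It adds that widget to the UpdateCollectable vertical box in the player controller's WBInterface, then destroys the actor.
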(event `self.Launch Interact`
  (`parent.Launch Interact`)
  (bind _asbp_player_controller (cast `/Game/Blueprints/BP_PlayerController` (`GameplayStatics.GetPlayerController` 0)))
  (bind _returnvalue (`|CreateWidget` "/Game/Blueprints/Widgets/WB_AddCollectectable.WB_AddCollectectable_C" null (`self.Type Content`) (`self.Number Content`)))
  (`VerticalBox.AddChildToVerticalBox` (`/Game/Blueprints/Widgets/BP_Interface_Player.UpdateCollectable` (`/Game/Blueprints/BP_PlayerController.WB_Interface` _asbp_player_controller)) _returnvalue)
  (`self.K2_DestroyActor`))

(fn `UserConstructionScript`
  (`parent.UserConstructionScript`))