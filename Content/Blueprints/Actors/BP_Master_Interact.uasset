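; Base interactable actor that shows proximity feedback to the player and accepts an interaction when in range.
; Sphere1, evidently the outer range, toggles the VisualInteract marker, while the inner Sphere swaps it for the Input prompt and sets CanInteract.
; A debug F key event calls LaunchInteract when CanInteract is true; here that event only hides the prompt, leaving CanInteract unchanged.
; Both spheres respond only to player character 0.
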(event OnComponentBeginOverlap(Sphere)
  (params (OverlappedComponent :type Primitive%20Component%20Object%20Reference) (OtherActor :type Actor%20Object%20Reference) (OtherComp :type Primitive%20Component%20Object%20Reference) (OtherBodyIndex :type Integer) (bFromSweep :type Boolean) (SweepResult :type Hit%20Result%20Structure%20%28by%20ref%29))
  (if (== OtherActor (Game|GetPlayerCharacter 0))
    (Variables|Default|SetCanInteract true)
    (Development|PrintString "Can Interact ")
    (Rendering|SetVisibility (Variables|Default|GetInput) true false)
    (Rendering|SetVisibility (Variables|Default|GetVisualInteract) false false)))

(event OnComponentEndOverlap(Sphere)
  (params (OverlappedComponent :type Primitive%20Component%20Object%20Reference) (OtherActor :type Actor%20Object%20Reference) (OtherComp :type Primitive%20Component%20Object%20Reference) (OtherBodyIndex :type Integer))
  (if (== OtherActor (Game|GetPlayerCharacter 0))
    (Variables|Default|SetCanInteract false)
    (Development|PrintString "can't interact")
    (Rendering|SetVisibility (Variables|Default|GetInput) false false)
    (Rendering|SetVisibility (Variables|Default|GetVisualInteract) true false)))

(event OnComponentBeginOverlap(Sphere1)
  (params (OverlappedComponent :type Primitive%20Component%20Object%20Reference) (OtherActor :type Actor%20Object%20Reference) (OtherComp :type Primitive%20Component%20Object%20Reference) (OtherBodyIndex :type Integer) (bFromSweep :type Boolean) (SweepResult :type Hit%20Result%20Structure%20%28by%20ref%29))
  (if (== OtherActor (Game|GetPlayerCharacter 0))
    (Rendering|SetVisibility (Variables|Default|GetVisualInteract) true false)))

(event OnComponentEndOverlap(Sphere1)
  (params (OverlappedComponent :type Primitive%20Component%20Object%20Reference) (OtherActor :type Actor%20Object%20Reference) (OtherComp :type Primitive%20Component%20Object%20Reference) (OtherBodyIndex :type Integer))
  (if (== OtherActor (Game|GetPlayerCharacter 0))
    (Rendering|SetVisibility (Variables|Default|GetVisualInteract) false false)))

(event Custom|Launch%20Interact
  (Rendering|SetVisibility (Variables|Default|GetInput) false false))

(event Input|KeyboardEvents|DebugKeyF
  (params (Key :type Key%20Structure :default "None") (ActionValue :type Input%20Action%20Value%20Structure))
  (:Pressed
    (if (Variables|Default|GetCanInteract)
      (CallFunction|LaunchInteract))))

(fn ConstructionScript)