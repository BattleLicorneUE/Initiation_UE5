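; AC_CharacterLogic is an actor component that tracks health for its owning Character and applies damage to it.
; On BeginPlay it caches the owner as a Character and sets Health from a character data asset's default.
; ApplyDamagesToCharacter subtracts damage through UpdateHealth, which clamps Health and reports when it reaches zero.
; The zero-health result has no follow-up logic, and the hit location and bone inputs are unused.
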(event `self.ReceiveBeginPlay`
  (`self.Init Ref`))

(event `Apply Damages To Character`
  (params (Damages :type "Float (double-precision)") (Location :type "Vector Structure") (Bones :type Name))
  (bind _actor_is_dead (`self.Update Health` Damages))
  (if _actor_is_dead
    _))

(fn `Init Ref`
  (bind _ascharacter (cast `Character` (`self.GetOwner`)))
  (set `self.Owner Character` _ascharacter)
  (set `self.Health` (`/Game/Blueprints/ActorsComponents/DataAssets/MasterDataAssets/BP_DataAssets_Character.Health Default` (`self.Data Assets Character`))))

(fn `Update Health`
  (params (Damages :type "Float (double-precision)"))
  (returns (`Actor is Dead` :type Boolean))
  (set `self.Health` (`KismetMathLibrary.FClamp` (- (`self.Health`) Damages) 0.0 9999.0))
  (if (<= (`self.Health`) 0.0)
    (return true)
    (else
      (return false))))